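; DoomsdayCosoCheVolaMockup is a mockup flying object for the Doomsday event.
; DoomsdayUnleashed reveals its mesh, then a timeline moves it from its current location to TargetPos over ArriveTime.
; After a LastingTime delay, a second timeline moves it on to FlyAwayPos over FlyAwayTime.
; Tick continuously applies random local rotation jitter on all axes, scaled by MinMaxRot and delta time.
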(event EventBeginPlay)

(event EventActorBeginOverlap
  (params (OtherActor :type Actor%20Object%20Reference)))

(event EventTick
  (params (DeltaSeconds :type Float%20%28single-precision%29))
  (bind _minmaxrot (Variables|Default|GetMinMaxRot))
  (bind _returnvalue (* DeltaSeconds _minmaxrot))
  (bind _returnvalue_2 (* DeltaSeconds _minmaxrot))
  (bind _returnvalue_3 (* DeltaSeconds _minmaxrot))
  (Transformation|AddActorLocalRotation (Math|Rotator|MakeRotator (Math|Random|RandomFloatinRange (* _returnvalue_3 -1.0) _returnvalue_3) (Math|Random|RandomFloatinRange (* _returnvalue_2 -1.0) _returnvalue_2) (Math|Random|RandomFloatinRange (* _returnvalue -1.0) _returnvalue)) false false))

(event EventDoomsdayUnleashed
  (Development|SetHiddeninGame (Variables|Default|GetStaticMesh) false false)
  (Components|Timeline|SetPlayRate (Variables|Default|GetAB) (/ 1.0 (Variables|Default|GetArriveTime)))
  (Variables|Default|SetStartingPos (Transformation|GetActorLocation))
  (bind _alpha (Timeline|AB Play)
    (:Update
      (Transformation|SetActorLocation (Math|Vector|Lerp(Vector) (Variables|Default|GetStartingPos) (Variables|Default|GetTargetPos) _alpha) false true))
    (:Finished
      (Utilities|FlowControl|Delay (Variables|Default|GetLastingTime))
      (Components|Timeline|SetPlayRate (Variables|Default|GetAB1) (/ 1.0 (Variables|Default|GetFlyAwayTime)))
      (bind _alpha_2 (Timeline|AB1 Play)
        (:Update
          (Transformation|SetActorLocation (Math|Vector|Lerp(Vector) (Variables|Default|GetTargetPos) (Variables|Default|GetFlyAwayPos) _alpha_2) false true))))))

(fn ConstructionScript
  (|CallParentFunction))