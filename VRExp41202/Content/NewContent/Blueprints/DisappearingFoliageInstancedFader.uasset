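; An instanced foliage mesh Blueprint whose instances disappear around the player as a fade progresses.
; On BeginPlay it registers itself in the DisappearingFoliage array of the first FaderActivator in the level.
; SeekAndDestroy permanently removes instances inside a world-space sphere at the player pawn, with a power-curve radius that grows as Onezero drops from one to zero.
; The pawn location stands in for the camera position, flagged as tech debt.
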(event Custom|SeekAndDestroy
  (params (onezero :type Float%20%28single-precision%29))
  (Class|HierarchicalInstancedStaticMeshComponent|RemoveInstances (Class|InstancedStaticMeshComponent|GetInstancesOverlappingSphere (Transformation|GetActorLocation (Pawn|GetControlledPawn (Game|GetPlayerController 0))) (* (Math|Float|Power (- 1.0 onezero) (Variables|Default|GetExponentialForFalloffSync)) (Variables|Default|GetFloatMultiplier)) true)))

(event EventBeginPlay
  (bind _outactors (Actor|GetAllActorsOfClass "/Game/NewContent/Blueprints/FaderActivator.FaderActivator_C"))
  (Utilities|Array|AddUnique (Variables|/Game/NewContent/Blueprints/FaderActivator.FaderActivator_C|GetDisappearingFoliage (Utilities|Array|Get(acopy) _outactors)) self))