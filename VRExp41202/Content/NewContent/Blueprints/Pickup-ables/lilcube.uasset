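; A physics pickup cube that attaches to a passed-in scene component when picked up and detaches to resume physics when laid down.
; The first pickup also calls STartDoomCycle on the player's Vive_Pawn2, then waits FadeDelay.
; It then puts PickupFader dynamic materials on its four meshes, and a Fader timeline animates their "op" parameter.
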(event EventBeginPlay)

(event EventActorBeginOverlap
  (params (OtherActor :type Actor%20Object%20Reference)))

(event EventGetPickedUp
  (params (Scene :type Scene%20Component%20Object%20Reference))
  (Variables|Default|SetBound Scene)
  (Physics|SetSimulatePhysics (Variables|Default|GetBody) false)
  (Class|Actor|AttachRootComponentto (Variables|Default|GetBound) "None" "KeepWorldPosition" true)
  (Utilities|FlowControl|DoOnce false
    (:Completed
      (bind _asvive_pawn_2 (Utilities|Casting|CastToVive_Pawn2 (Pawn|GetControlledPawn (Game|GetPlayerController 0))))
      (Default|STartDoomCycle _asvive_pawn_2)
      (Utilities|FlowControl|Delay (Variables|Default|GetFadeDelay))
      (bind _returnvalue (Rendering|Material|CreateDynamicMaterialInstance (Variables|Default|GetBody) 0 "/Game/ToSettle/Materials/PickupFader.PickupFader" :!class /Script/Engine.PrimitiveComponent))
      (Utilities|Array|AddUnique (Variables|Default|GetInstances) _returnvalue)
      (bind _returnvalue_2 (Rendering|Material|CreateDynamicMaterialInstance (Variables|Default|GetStaticMesh) 0 "/Game/ToSettle/Materials/PickupFader.PickupFader" :!class /Script/Engine.PrimitiveComponent))
      (Utilities|Array|AddUnique (Variables|Default|GetInstances) _returnvalue_2)
      (bind _returnvalue_3 (Rendering|Material|CreateDynamicMaterialInstance (Variables|Default|GetStaticMesh1) 0 "/Game/ToSettle/Materials/PickupFader.PickupFader" :!class /Script/Engine.PrimitiveComponent))
      (Utilities|Array|AddUnique (Variables|Default|GetInstances) _returnvalue_3)
      (bind _returnvalue_4 (Rendering|Material|CreateDynamicMaterialInstance (Variables|Default|GetStaticMesh2) 0 "/Game/ToSettle/Materials/PickupFader.PickupFader" :!class /Script/Engine.PrimitiveComponent))
      (Utilities|Array|AddUnique (Variables|Default|GetInstances) _returnvalue_4)
      (bind _alpha (Timeline|Fader Play)
        (:Update
          (for _array_element (Variables|Default|GetInstances)
            (Rendering|Material|SetScalarParameterValue _array_element "op" _alpha :!class /Script/Engine.MaterialInstanceDynamic)))))))

(event EventGetLaidDown
  (params (Scene :type Scene%20Component%20Object%20Reference))
  (Class|Actor|DetachRootComponentfromParent true)
  (Physics|SetSimulatePhysics (Variables|Default|GetBody) true))

(fn ConstructionScript
  (|CallParentFunction))