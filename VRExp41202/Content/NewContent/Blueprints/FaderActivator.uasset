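; FaderActivator is an actor that runs a timed fade for an opacity parameter and disappearing foliage when play begins.
; On BeginPlay it scales the Fade timeline's play rate by TotalFadeTime, then plays it.
; Each update writes the OneZero track into the OpFaderParam material parameter collection and passes it to SeekAndDestroy on every DisappearingFoliage entry.
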(event Custom|InitVariables
  (bind _fade (Variables|Default|GetFade))
  (Utilities|FlowControl|Sequence
    (:then_1
      (Components|Timeline|SetPlayRate _fade (/ (Components|Animation|GetPlayRate _fade) (Variables|Default|GetTotalFadeTime))))))

(event Custom|GameplayActions
  (bind _onezero (Timeline|Fade Play)
    (:Update
      (Rendering|Material|SetScalarParameterValue "/Game/NewContent/Materials/OpFaderParam.OpFaderParam" "onezero" _onezero :!class /Script/Engine.KismetMaterialLibrary)
      (for _array_element (Variables|Default|GetDisappearingFoliage)
        (Default|SeekandDestroy _array_element _onezero)))))

(event EventBeginPlay
  (CallFunction|InitVariables)
  (CallFunction|GameplayActions))

(event Collision|EventActorBeginOverlap
  (params (OtherActor :type Actor%20Object%20Reference)))

(fn ConstructionScript)