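; Spatialized sound actor that plays the audio crescendo for the Doomsday buildup.
; When DoomsdayUnleashed fires, it starts its Audio component and a timeline whose volume track drives the volume multiplier on each update.
; The timeline's play rate is the inverse of BuildupTime, so a normalized curve can stretch to the buildup duration.
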(event EventBeginPlay)

(event Collision|EventActorBeginOverlap
  (params (OtherActor :type Actor%20Object%20Reference)))

(event EventTick
  (params (DeltaSeconds :type Float%20%28single-precision%29)))

(event EventDoomsdayUnleashed
  (Audio|Components|Audio|Play (Variables|Default|GetAudio) 0.0)
  (Components|Timeline|SetPlayRate (Variables|Default|GetSoundTimeline) (/ 1.0 (Variables|Default|GetBuildupTime)))
  ;[1 1 1] Freeze!
  (bind _volumetrack (Timeline|SoundTimeline Play)
    (:Update
      (Audio|Components|Audio|SetVolumeMultiplier (Variables|Default|GetAudio) _volumetrack :!class /Script/Engine.AudioComponent))))

(fn ConstructionScript
  (|CallParentFunction))