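; Doomsday fog Blueprint that fades a referenced Exponential Height Fog to a final inscattering color as soon as play begins.
; BeginPlay caches the fog's starting values, then runs a timeline with play rate scaled by FadeTime to lerp the color.
; The start color comes from DirectionalInscatteringColor, although the fade writes FogInscatteringColor.
; Density and start-distance fades are present but disconnected, so only color changes.
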(event Custom|InitVariables
  (bind _expheightfog (Variables|Default|GetExpHeightFog))
  (bind _component (Variables|/Script/Engine.ExponentialHeightFog|GetComponent _expheightfog))
  (Utilities|FlowControl|Sequence
    (:then_0
      (Variables|Default|SetInitialFogDensity (Variables|/Script/Engine.ExponentialHeightFogComponent|GetFogDensity _component)))
    (:then_1
      (Variables|Default|SetInitialFogStartDistance (Variables|/Script/Engine.ExponentialHeightFogComponent|GetStartDistance _component)))
    (:then_2
      (Variables|Default|SetInitialInscatteringColor (Variables|/Script/Engine.ExponentialHeightFogComponent|GetDirectionalInscatteringColor _component)))))

(event EventBeginPlay
  (CallFunction|InitVariables)
  (CallFunction|DoomsdayUnleashed))

(event EventDoomsdayUnleashed
  (Components|Timeline|SetPlayRate (Variables|Default|GetFogTimeline) (/ 1.0 (Variables|Default|GetFadeTime)))
  (bind _lerp (Timeline|FogTimeline Play)
    (:Update
      (Class|ExponentialHeightFogComponent|SetFogInscatteringColor (Variables|/Script/Engine.ExponentialHeightFog|GetComponent (Variables|Default|GetExpHeightFog)) (Math|Color|Lerp(LinearColor) (Variables|Default|GetInitialInscatteringColor) (Variables|Default|GetFinalInscatteringColor) _lerp)))))

(fn ConstructionScript
  (|CallParentFunction))