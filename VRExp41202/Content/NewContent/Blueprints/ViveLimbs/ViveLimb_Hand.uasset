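; ViveLimb_Hand is a hand limb Blueprint for Vive controllers that picks up objects.
; On trigger press, it takes the first PickupAble actor overlapping the HandWIP component, calls GetPickedUp with that component and stores it as AttachedActor.
; Trigger release is empty, and the GetLaidDown drop logic for the stored actor is unconnected, so it never runs.
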(event EventViveTriggerPress
  (bind _hand__wip_ (Variables|Default|GetHand%20%28WIP%29))
  (bind _overlappingactors (Collision|GetOverlappingActors _hand__wip_ "/Game/NewContent/Blueprints/Pickup-ables/Pickup-Able.Pickup-Able_C" :!class /Script/Engine.PrimitiveComponent))
  (bind _item (Utilities|Array|Get(acopy) _overlappingactors))
  (if (> (Utilities|Array|Length _overlappingactors) 0)
    (bind _aspickup__able (Utilities|Casting|CastToPickup-Able _item))
    (Default|GetPickedUp _aspickup__able (Variables|Default|GetHand%20%28WIP%29))
    (Variables|Default|SetAttached%20Actor _item)))

(event EventViveTriggerRelease)

(fn ConstructionScript
  (|CallParentFunction))