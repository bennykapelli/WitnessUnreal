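; DoomsdayUDS shifts the UDS sky actor's time of day between two set values for the Doomsday sequence.
; A timeline, its play rate scaled so the blend lasts Time, lerps TimeOfDay from A to B.
; It plays on BeginPlay after an empty InitVariables event, and again on DoomsdayUnleashed.
; The construction script applies either endpoint, chosen by IsA, as an editor preview when UDS is valid.
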(event Custom|InitVariables)

(event EventBeginPlay
  (CallFunction|InitVariables)
  (Components|Timeline|SetPlayRate (Variables|Default|GetUDSTimeline) (/ 1.0 (Variables|Default|GetTime)))
  (bind _lerp (Timeline|UDSTimeline Play)
    (:Update
      (Variables|/Game/UltraDynamicSky/Blueprints/Ultra_Dynamic_Sky_BP.Ultra_Dynamic_Sky_BP_C|SetTime%20of%20Day (Variables|Default|GetUDS) (Math|Float|Lerp (Variables|Default|GetTimeOfDayA) (Variables|Default|GetTimeOfDayB) _lerp)))))

(event EventDoomsdayUnleashed
  (Components|Timeline|SetPlayRate (Variables|Default|GetUDSTimeline) (/ 1.0 (Variables|Default|GetTime)))
  (bind _lerp (Timeline|UDSTimeline Play)
    (:Update
      (Variables|/Game/UltraDynamicSky/Blueprints/Ultra_Dynamic_Sky_BP.Ultra_Dynamic_Sky_BP_C|SetTime%20of%20Day (Variables|Default|GetUDS) (Math|Float|Lerp (Variables|Default|GetTimeOfDayA) (Variables|Default|GetTimeOfDayB) _lerp)))))

(fn ConstructionScript
  (|CallParentFunction)
  (Utilities|IsValid (Variables|Default|GetUDS)
    (:Is%20Valid
      (if (Variables|Default|GetIsA)
        (Variables|/Game/UltraDynamicSky/Blueprints/Ultra_Dynamic_Sky_BP.Ultra_Dynamic_Sky_BP_C|SetTime%20of%20Day (Variables|Default|GetUDS) (Variables|Default|GetTimeOfDayA))
        (else
          (Variables|/Game/UltraDynamicSky/Blueprints/Ultra_Dynamic_Sky_BP.Ultra_Dynamic_Sky_BP_C|SetTime%20of%20Day (Variables|Default|GetUDS) (Variables|Default|GetTimeOfDayB)))))))