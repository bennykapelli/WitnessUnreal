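; Vive VR controller limb that lets the player teleport by holding and releasing the thumbstick, with empty trigger events.
; Initialize stores the owning master and its motion controller.
; While teleporting, Tick draws a debug line trace from TeleportOrientation, marked for removal before release.
; Release re-traces and, only on a hit, moves the master's room root, subtracting the head's horizontal offset, and clears the teleporting state.
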(event Custom|ViveTriggerRelease)

(event Custom|ViveTriggerPress)

(event Custom|Initialize
  (params (Master :type Vive%20Pawn%202%20Object%20Reference) (MyMotionController :type Motion%20Controller%20Component%20Object%20Reference))
  (Variables|Default|SetMastah Master)
  (Variables|Default|SetMyMotionController MyMotionController))

(event Custom|Draw%20Teleport%20Preview
  (bind _teleportorientation (Variables|Default|GetTeleportOrientation))
  (bind _returnvalue (Transformation|GetWorldLocation _teleportorientation))
  (bind _returnvalue_2 (Transformation|GetWorldRotation _teleportorientation))
  (bind _returnvalue_3 (Math|Vector|GetForwardVector _returnvalue_2))
  ;[1 1 1] KEEPING THISFOR DEBUGGING, MUST REMOVE BEFORE RELEASE
  (Collision|LineTraceByChannel (+ _returnvalue _returnvalue_3) (+ _returnvalue (* _returnvalue_3 (Variables|/Game/GamePlayerModes/Player/Vive_Pawn2.Vive_Pawn2_C|GetTeleport_Range (Variables|Default|GetMastah)))) "TraceTypeQuery1" false 0 "ForOneFrame") ; ray trace to a new teleport location
)

(event Custom|ViveThumbstickRelease
  (bind _mastah (Variables|Default|GetMastah))
  (bind _teleportorientation (Variables|Default|GetTeleportOrientation))
  (bind _returnvalue (Transformation|GetWorldLocation _teleportorientation))
  (bind _returnvalue_2 (Transformation|GetWorldRotation _teleportorientation))
  (bind _head (Variables|/Game/GamePlayerModes/Player/Vive_Pawn2.Vive_Pawn2_C|GetHead _mastah))
  (bind _defaultsceneroot (Variables|/Game/GamePlayerModes/Player/Vive_Pawn2.Vive_Pawn2_C|GetDefaultSceneRoot _mastah))
  (bind _returnvalue_3 (Math|Vector|GetForwardVector _returnvalue_2))
  (bind _returnvalue_4 (Transformation|GetWorldLocation _head))
  (bind _returnvalue_5 (Transformation|GetWorldLocation _defaultsceneroot))
  (bind _returnvalue_6 (- _returnvalue_4 _returnvalue_5))
  (bind (_x _y) (Math|Vector|BreakVector _returnvalue_6))
  ;[1 1 1] KEEPING THISFOR DEBUGGING, MUST REMOVE BEFORE RELEASE
  (bind (_outhit _returnvalue_7) (Collision|LineTraceByChannel (+ _returnvalue _returnvalue_3) (+ _returnvalue (* _returnvalue_3 (Variables|/Game/GamePlayerModes/Player/Vive_Pawn2.Vive_Pawn2_C|GetTeleport_Range (Variables|Default|GetMastah)))) "TraceTypeQuery1" false 0 "ForOneFrame")) ; ray trace to a new teleport location
  (if _returnvalue_7 ; only do the stuff if you actually can teleport to somewhere
    (Transformation|SetWorldLocation (Variables|/Game/GamePlayerModes/Player/Vive_Pawn2.Vive_Pawn2_C|GetDefaultSceneRoot (Variables|Default|GetMastah)) (- (.Location (Collision|BreakHitResult _outhit)) (Math|Vector|MakeVector _x _y 0.0)) false true) ; boom! teleport!
    (Variables|Default|SetTeleporting false)))

(event Custom|ViveThumbstickPress
  ;[1 1 1] KEEPING THISFOR DEBUGGING, MUST REMOVE BEFORE RELEASE
  (Variables|Default|SetTeleporting true))

(event EventBeginPlay)

(event EventActorBeginOverlap
  (params (OtherActor :type Actor%20Object%20Reference)))

(event EventTick
  (params (DeltaSeconds :type Float%20%28single-precision%29)))

(event EventTick
  (params (DeltaSeconds :type Float%20%28single-precision%29))
  ;[1 1 1] KEEPING THISFOR DEBUGGING, MUST REMOVE BEFORE RELEASE
  (if (Variables|Default|GetTeleporting)
    (CallFunction|DrawTeleportPreview)))

(fn ConstructionScript)